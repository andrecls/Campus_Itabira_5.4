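; Weather controller actor that drives level lighting from live OpenWeatherMap data for Itabira.
; A looping timer started on BeginPlay sends a VaRest GET request every few seconds and reads the main weather condition.
; Clear, Clouds and Rain each set preset DirectionalLight and SkyLight intensities.
; Rain also spawns a new water-dripping emitter high above the player on each poll, with no cleanup here.
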(event `self.ReceiveBeginPlay`
  (`KismetSystemLibrary.K2_SetTimerDelegate` (delegate `ChamarAPI_clima`) 5.0 true))

(event `ChamarAPI_clima`
  (bind _returnvalue (`VaRestSubsystem.ConstructVaRestRequestExt` (subsystem `VaRestSubsystem`) "GET" "x_www_form_urlencoded_url"))
  (bind _result (`VaRestRequestJSON.ApplyURL` _returnvalue "https://api.openweathermap.org/data/2.5/weather?q=Itabira&appid=b4d49c46372677f0027c273be10f0d7f&units=metric"))
  (bind _returnvalue_2 (`VaRestJsonValue.AsObject` (`|GetArrayItem` (`VaRestJsonObject.GetArrayField` _result "weather"))))
  (switch `string` (`VaRestJsonObject.GetStringField` _returnvalue_2 "main")
    (:`Clear`
      (bind _returnvalue_3 (`GameplayStatics.GetActorOfClass` "/Script/Engine.DirectionalLight"))
      (`LightComponent.SetIntensity` (`Light.LightComponent` _returnvalue_3) 10.0)
      (bind _returnvalue_4 (`GameplayStatics.GetActorOfClass` "/Script/Engine.SkyLight"))
      (`SkyLightComponent.SetIntensity` (`SkyLight.LightComponent` _returnvalue_4) 1.5))
    (:`Clouds`
      (bind _returnvalue_5 (`GameplayStatics.GetActorOfClass` "/Script/Engine.DirectionalLight"))
      (`LightComponent.SetIntensity` (`Light.LightComponent` _returnvalue_5) 2.0)
      (bind _returnvalue_6 (`GameplayStatics.GetActorOfClass` "/Script/Engine.SkyLight"))
      (`SkyLightComponent.SetIntensity` (`SkyLight.LightComponent` _returnvalue_6) 0.75))
    (:`Rain`
      (bind _returnvalue_7 (`GameplayStatics.GetActorOfClass` "/Script/Engine.DirectionalLight"))
      (`LightComponent.SetIntensity` (`Light.LightComponent` _returnvalue_7) 0.2)
      (bind _returnvalue_8 (`GameplayStatics.GetActorOfClass` "/Script/Engine.SkyLight"))
      (`SkyLightComponent.SetIntensity` (`SkyLight.LightComponent` _returnvalue_8) 0.3)
      (`GameplayStatics.SpawnEmitterAtLocation` "/Game/Realistic_Starter_VFX_Pack_Vol2/Particles/Water/P_Water_Dripping_B.P_Water_Dripping_B" (+ (`self.K2_GetActorLocation` (`GameplayStatics.GetPlayerCharacter` 0)) (0.0 0.0 1000.0))))))

(fn `UserConstructionScript`)