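; BP_Poste is a lamp post whose point light turns on at night and off during the day.
; On BeginPlay, a looping five-second timer calls ChecarLuz.
; ChecarLuz reads the current hour from the system clock via Now and shows the light between 18:00 and 06:00, hiding it otherwise.
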(event `self.ReceiveBeginPlay`
  (`KismetSystemLibrary.K2_SetTimerDelegate` (delegate `ChecarLuz`) 5.0 true))

(event `ChecarLuz`
  (bind _pointlight (`self.PointLight`))
  (bind (_year _month _day _hour) (`KismetMathLibrary.BreakDateTime` (`KismetMathLibrary.Now`)))
  (if (or (< _hour 6) (>= _hour 18))
    (`SceneComponent.SetVisibility` _pointlight true false)
    (else
      (`SceneComponent.SetVisibility` _pointlight false false))))

(fn `UserConstructionScript`)