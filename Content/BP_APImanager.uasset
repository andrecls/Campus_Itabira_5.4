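; BP_APImanager is an actor that fills an in-world events board with notices fetched from a UNIFEI dashboard web API.
; On BeginPlay it sends a VaRest GET request, then wraps the returned JSON array in a "lista" object so it can be decoded.
; Each entry becomes a WBP_EventoCard with title and content, added to the notice box of the WBP_MuralEventos shown by its widget component.
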(event `self.ReceiveBeginPlay`
  (bind _returnvalue (`VaRestSubsystem.ConstructVaRestRequestExt` (subsystem `VaRestSubsystem`) "GET" "x_www_form_urlencoded_url"))
  (add `VaRestRequestJSON.OnRequestComplete` _returnvalue (delegate `AoReceberDados`))
  (`VaRestRequestJSON.ProcessURL` _returnvalue "https://dashboard-unifei.onrender.com/api/dados"))

(event `AoReceberDados`
  (params (Request :type "VaRestRequestJSON Object Reference"))
  (bind _returnvalue (`VaRestRequestJSON.GetResponseContentAsString` Request true))
  (bind _returnvalue_2 (`VaRestSubsystem.ConstructVaRestJsonObject` (subsystem `VaRestSubsystem`)))
  (`VaRestJsonObject.DecodeJson` _returnvalue_2 (`KismetStringLibrary.Concat_StrStr` "{\"lista\": " _returnvalue "}") true)
  (for _array_element (`VaRestJsonObject.GetObjectArrayField` _returnvalue_2 "lista")
    (bind _returnvalue_3 (`|CreateWidget` "/Game/WBP_EventoCard.WBP_EventoCard_C"))
    (set `TextBlock.Text` (`KismetTextLibrary.Conv_StringToText` (`VaRestJsonObject.GetStringField` _array_element "titulo")) (`/Game/WBP_EventoCard.Text_titulo` _returnvalue_3))
    (set `TextBlock.Text` (`KismetTextLibrary.Conv_StringToText` (`VaRestJsonObject.GetStringField` _array_element "conteudo")) (`/Game/WBP_EventoCard.Text_conteudo` _returnvalue_3))
    (bind _aswbp_mural_eventos (cast `/Game/WBP_MuralEventos` (`WidgetComponent.GetUserWidgetObject` (`self.Widget`))))
    (`PanelWidget.AddChild` (`/Game/WBP_MuralEventos.CaixaDeAvisos` _aswbp_mural_eventos) _returnvalue_3)))

(fn `UserConstructionScript`)